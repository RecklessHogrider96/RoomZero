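; BP_ItemObject wraps an ItemData record for a single item that has a quantity and a width and height on a grid.
; Simple getters expose the whole record, its ItemID as the name, its quantity, and its icon paired with a rotation flag.
; GetDimensions returns the stored grid width and height as they are, without swapping them for rotation.
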(fn GetName
  (return (.ItemID (Utilities|Struct|BreakFInventoryEntry (Variables|Default|GetItemData)))))

(fn GetQuantity
  (return (.Quantity (Utilities|Struct|BreakFInventoryEntry (Variables|Default|GetItemData)))))

(fn GetIcon
  (bind _itemdata (Variables|Default|GetItemData))
  (bind (_itemid _itemtype _quantity _weight _gridwidth _gridheight _rotated _icon) (Utilities|Struct|BreakFInventoryEntry _itemdata))
  (return _rotated _icon))

(fn GetItem
  (return (Variables|Default|GetItemData)))

(fn GetDimensions
  (bind _itemdata (Variables|Default|GetItemData))
  (return (Utilities|Struct|MakeIntPoint (.gridwidth _itemdata) (.gridheight _itemdata))))