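; Game instance for Room Zero that holds the player's stash and loadout inventories as maps of item entries keyed by item ID.
; AddItemToStash and AddItemToLoadout stack quantity onto an existing entry, keeping its other fields and grid position, or insert the item as new.
; Init seeds the stash with hard-coded key items at grid positions, then adds a duplicate key through AddItemToStash, which stacks it.
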(event EventInit
  (bind _returnvalue (Utilities|Name|MakeLiteralName "Key0"))
  (bind _returnvalue_2 (Utilities|Name|MakeLiteralName "Key1"))
  (bind _returnvalue_3 (Utilities|Name|MakeLiteralName "Key2"))
  (bind _output_get (Variables|Default|SetStashInventory (Utilities|Map|MakeMap _returnvalue (Utilities|Struct|MakeFInventoryEntry _returnvalue "NewEnumerator0" 1))))
  (Utilities|Map|Add _output_get _returnvalue_2 (Utilities|Struct|MakeFInventoryEntry _returnvalue_2 "NewEnumerator0" 1 0.0 1 1 "(X=0.000000,Y=1.000000)"))
  (Utilities|Map|Add _output_get _returnvalue_3 (Utilities|Struct|MakeFInventoryEntry _returnvalue_3 "NewEnumerator0" 1 0.0 1 1 "(X=0.000000,Y=2.000000)"))
  (CallFunction|AddItemtoStash (Utilities|Struct|MakeFInventoryEntry (Utilities|Name|MakeLiteralName "Key2") "NewEnumerator0" 1 0.0 1 1 "(X=0.000000,Y=2.000000)")))

(fn AddItemtoStash
  (params (Item :type F%20Inventory%20Entry%20Structure))
  (bind (_itemid _itemtype _quantity) (Utilities|Struct|BreakFInventoryEntry Item))
  (bind _stashinventory (Variables|Default|GetStashInventory))
  (bind _value (Utilities|Map|Find _stashinventory _itemid))
  (bind (_itemid_2 _itemtype_2 _quantity_2 _weight _gridwidth _gridheight _gridposition) (Utilities|Struct|BreakFInventoryEntry _value))
  (if (Utilities|Map|Contains _stashinventory _itemid)
    (Utilities|Map|Add _stashinventory _itemid_2 (Utilities|Struct|MakeFInventoryEntry _itemid_2 _itemtype_2 (+ _quantity_2 _quantity) _weight _gridwidth _gridheight _gridposition))
    (else
      (Utilities|Map|Add _stashinventory _itemid Item))))

(fn AddItemtoLoadout
  (params (Item :type F%20Inventory%20Entry%20Structure))
  (bind (_itemid _itemtype _quantity) (Utilities|Struct|BreakFInventoryEntry Item))
  (bind _loadoutinventory (Variables|Default|GetLoadoutInventory))
  (bind _value (Utilities|Map|Find _loadoutinventory _itemid))
  (bind (_itemid_2 _itemtype_2 _quantity_2 _weight _gridwidth _gridheight _gridposition) (Utilities|Struct|BreakFInventoryEntry _value))
  (if (Utilities|Map|Contains _loadoutinventory _itemid)
    (Utilities|Map|Add _loadoutinventory _itemid_2 (Utilities|Struct|MakeFInventoryEntry _itemid_2 _itemtype_2 (+ _quantity_2 _quantity) _weight _gridwidth _gridheight _gridposition))
    (else
      (Utilities|Map|Add _loadoutinventory _itemid Item))))