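; Game instance for Room Zero that holds the player's stash and loadout inventories.
; Each inventory is a map of FInventoryEntry keyed by ItemID, with functions to add, fetch and remove entries.
; Adding an existing ID rebuilds its entry with the summed quantity, and loadout adds also record the result in AddedItem.
; A lookup reports whether a key is in the loadout and its quantity.
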(event EventInit)

(fn AddItemtoStash
  (params (Item :type F%20Inventory%20Entry%20Structure))
  (bind (_itemid _itemtype _quantity) (Utilities|Struct|BreakFInventoryEntry Item))
  (bind _stashinventory (Variables|Default|GetStashInventory))
  (bind _value (Utilities|Map|Find _stashinventory _itemid))
  (bind (_itemid_2 _itemtype_2 _quantity_2 _weight _gridwidth _gridheight _rotated _icon _gridposition) (Utilities|Struct|BreakFInventoryEntry _value))
  (if (Utilities|Map|Contains _stashinventory _itemid)
    (Utilities|Map|Add _stashinventory _itemid_2 (Utilities|Struct|MakeFInventoryEntry _itemid_2 _itemtype_2 (+ _quantity_2 _quantity) _weight _gridwidth _gridheight _rotated _icon _gridposition))
    (else
      (Utilities|Map|Add _stashinventory _itemid Item))))

(fn AddItemtoLoadout
  (params (Item :type F%20Inventory%20Entry%20Structure))
  (bind (_itemid _itemtype _quantity) (Utilities|Struct|BreakFInventoryEntry Item))
  (bind _loadoutinventory (Variables|Default|GetLoadoutInventory))
  (bind _value (Utilities|Map|Find _loadoutinventory _itemid))
  (bind (_itemid_2 _itemtype_2 _quantity_2 _weight _gridwidth _gridheight _rotated _icon _gridposition) (Utilities|Struct|BreakFInventoryEntry _value))
  (bind _returnvalue (+ _quantity_2 _quantity))
  (bind _finventoryentry (Utilities|Struct|MakeFInventoryEntry _itemid_2 _itemtype_2 _returnvalue _weight _gridwidth _gridheight _rotated _icon _gridposition))
  (if (Utilities|Map|Contains _loadoutinventory _itemid)
    (Utilities|Map|Add _loadoutinventory _itemid_2 _finventoryentry)
    (LocalVariables|SetAddedItem _finventoryentry)
    (else
      (Utilities|Map|Add _loadoutinventory _itemid Item)
      (LocalVariables|SetAddedItem Item))))

(fn FetchStash
  (return (Variables|Default|GetStashInventory)))

(fn FetchLoadout
  (return (Variables|Default|GetLoadoutInventory)))

(fn FindKeyinLoadout
  (params (KeyToSearch :type Name))
  (bind _loadoutinventory (Variables|Default|GetLoadoutInventory))
  (bind (_value _returnvalue) (Utilities|Map|Find _loadoutinventory KeyToSearch))
  (return _returnvalue (.quantity _value)))

(fn RemoveItemfromStash
  (params (ItemName :type Name))
  (Utilities|Map|Remove (Variables|Default|GetStashInventory) ItemName))

(fn RemoveItemfromLoadout
  (params (itemID :type Name))
  (Utilities|Map|Remove (Variables|Default|GetLoadoutInventory) itemID))