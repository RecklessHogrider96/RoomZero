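; BP_Lockable_Component is an actor component that makes its owner lockable and tracks whether it is unlocked.
; TryUnlock returns immediately if already unlocked, otherwise dispatches on UnlockMethod: Items, Code, Puzzle or Auto.
; Items requires every RequiredItems key in the game instance's loadout with positive quantity, without consuming it; Code compares input against the stored code.
; Auto always unlocks, while Puzzle returns an unset local flag, with no puzzle logic.
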(event EventBeginPlay)

(event EventTick
  (params (DeltaSeconds :type Float%20%28single-precision%29)))

(fn TryUnlock
  (params (InputCode :type String))
  (if (Variables|Public|GetbIsUnlocked)
    (return (Variables|Public|GetbIsUnlocked))
    (else
      (switch Utilities|FlowControl|Switch|SwitchonEUnlockMethod (Variables|Public|GetUnlockMethod)
        (:NewEnumerator0
          (bind _isunlocked (Private|TryUnlockbyItems))
          (Variables|Public|SetbIsUnlocked _isunlocked))
        (:NewEnumerator1
          (bind _isunlocked_2 (Private|TryUnlockbyCode InputCode))
          (Variables|Public|SetbIsUnlocked _isunlocked_2))
        (:NewEnumerator2
          (bind _isunlocked_3 (Private|TryUnlockbyPuzzle))
          (Variables|Public|SetbIsUnlocked _isunlocked_3))
        (:NewEnumerator3
          (Variables|Public|SetbIsUnlocked true)))
      (return (Variables|Public|GetbIsUnlocked)))))

(fn TryUnlockbyCode
  (params (InputCode :type String))
  (return (Utilities|Enum|Equal(Enum) InputCode (Variables|ForCodeUnlock|GetCode))))

(fn TryUnlockbyPuzzle
  (return (LocalVariables|GetisUnlocked%20%28local%29)))

(fn TryUnlockbyItems
  (LocalVariables|SetisUnlocked%20%28local%29 true)
  (bind _array_element (Utilities|Array|ForEachLoopwithBreak (Variables|ForItemUnlock|GetRequiredItems) :!label _label)
    (:LoopBody
      (bind (_iskeypresent _quantity) (Default|FindKeyinLoadout (.AsBP%20Room%20Zero%20Game%20Instance (Utilities|Casting|CastToBP_RoomZeroGameInstance (Game|GetGameInstance))) _array_element))
      (if _iskeypresent ; Chech if Key is in Loadout
        (if (not (> _quantity 0)) ; Check Quantity is more than 0
          (LocalVariables|SetisUnlocked%20%28local%29 false :!label _label_2)
          (goto _label Break))
        (else
          (goto _label_2))))
    (:Completed
      (return (LocalVariables|GetisUnlocked%20%28local%29)))))