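; BP_KeyItem is a pickup key that the player collects into the game's loadout inventory.
; Its box overlap registers the key as the third-person character's CurrentInteractable, and leaving the box clears it.
; PickupKey adds one entry under KeyName to LoadoutInventory on BP_RoomZeroGameInstance, prints debug messages, and destroys the actor.
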(event OnComponentBeginOverlap(Box)
  (params (OverlappedComponent :type Primitive%20Component%20Object%20Reference) (OtherActor :type Actor%20Object%20Reference) (OtherComp :type Primitive%20Component%20Object%20Reference) (OtherBodyIndex :type Integer) (bFromSweep :type Boolean) (SweepResult :type Hit%20Result%20Structure%20%28by%20ref%29))
  (if (Actor|ActorHasTag OtherActor "Player")
    (bind _asbp_third_person_character (Utilities|Casting|CastToBP_ThirdPersonCharacter OtherActor))
    (bind _output_get (Variables|Default|SetPlayerRef _asbp_third_person_character))
    (Development|PrintString "This is a Key!")
    (Variables|/Game/Blueprints/BP_ThirdPersonCharacter.BP_ThirdPersonCharacter_C|SetCurrentInteractable _output_get self)))

(event OnComponentEndOverlap(Box)
  (params (OverlappedComponent :type Primitive%20Component%20Object%20Reference) (OtherActor :type Actor%20Object%20Reference) (OtherComp :type Primitive%20Component%20Object%20Reference) (OtherBodyIndex :type Integer))
  (if (Actor|ActorHasTag OtherActor "Player")
    (Variables|/Game/Blueprints/BP_ThirdPersonCharacter.BP_ThirdPersonCharacter_C|SetCurrentInteractable (Variables|Default|GetPlayerRef) 0)))

(event Custom|PickupKey
  (bind _asbp_room_zero_game_instance (Utilities|Casting|CastToBP_RoomZeroGameInstance (Game|GetGameInstance))
    (:then
      (Utilities|Map|Add (Variables|/Game/BP_RoomZeroGameInstance.BP_RoomZeroGameInstance_C|GetLoadoutInventory _asbp_room_zero_game_instance) (Variables|Default|GetKeyName) (Utilities|Struct|MakeFInventoryEntry "0" "NewEnumerator0" 1))
      (Development|PrintString "Picked up key!")
      (Actor|DestroyActor))
    (:CastFailed
      (Development|PrintString "GameInstance Cast Fail!!!"))))

(event EventBeginPlay)

(event Collision|EventActorBeginOverlap
  (params (OtherActor :type Actor%20Object%20Reference)))

(event EventTick
  (params (DeltaSeconds :type Float%20%28single-precision%29)))

(fn ConstructionScript)