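; BP_Door is a key-gated door that ends the current level when the player has the required key.
; When anything overlaps DoorMesh, it checks whether the RoomZero game instance inventory contains RequiredKey.
; Without the key it prints a locked message; with it, it prints an unlocked message and opens the main menu level.
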(event OnComponentBeginOverlap(DoorMesh)
  (params (OverlappedComponent :type Primitive%20Component%20Object%20Reference) (OtherActor :type Actor%20Object%20Reference) (OtherComp :type Primitive%20Component%20Object%20Reference) (OtherBodyIndex :type Integer) (bFromSweep :type Boolean) (SweepResult :type Hit%20Result%20Structure%20%28by%20ref%29))
  (bind _asbp_room_zero_game_instance (Utilities|Casting|CastToBP_RoomZeroGameInstance (Game|GetGameInstance)))
  (bind _output_get (Variables|Default|SetisLocked (not (Utilities|Array|ContainsItem (Variables|/Game/BP_RoomZeroGameInstance.BP_RoomZeroGameInstance_C|GetInventory _asbp_room_zero_game_instance) (Variables|Default|GetrequiredKey)))))
  (if _output_get
    (Development|PrintString "You do not have the key!")
    (else
      (Development|PrintString "Door is unlocked!")
      (Game|OpenLevel(byObjectReference) "/Game/Levels/Level_MainMenu.Level_MainMenu"))))

(event EventBeginPlay)

(event Collision|EventActorBeginOverlap
  (params (OtherActor :type Actor%20Object%20Reference)))

(event EventTick
  (params (DeltaSeconds :type Float%20%28single-precision%29)))

(fn ConstructionScript)