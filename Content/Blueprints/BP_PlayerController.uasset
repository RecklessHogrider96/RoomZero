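; Player controller that sets up the local player's UI for the main menu, level or lobby, based on the game state class.
; In levels it creates the room HUD and inventory widget, then restores Key items from the GameInstance loadout into the InventoryComponent.
; It also shows pickup messages, toggles the inventory with matching input modes, and opens levels as listen servers through a console command.
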(event Custom|OpenLevelRoom
  (params (Level :type Soft%20World%20Reference%20Structure))
  (bind _worldasset (Utilities|Struct|BreakSoftWorldReference Level))
  (bind _returnvalue (Class|KismetSystemLibrary|ToSoftObjPath(SoftObjRef) _worldasset))
  (bind _pathstring (Utilities|BreakSoftObjectPath _returnvalue))
  (bind _returnvalue_2 (Utilities|String|ParseIntoArray _pathstring "."))
  (Development|ExecuteConsoleCommand (Utilities|String|Append "open " (Utilities|String|Append (Utilities|Array|Get(acopy) _returnvalue_2 (- (Utilities|Array|Length _returnvalue_2) 1)) "?listen")) 0))

(event Custom|ToggleInventory
  (if (UserInterface|Viewport|IsinViewport (Variables|Default|GetInventoryWidget))
    (Widget|RemovefromParent (Variables|Default|GetInventoryWidget))
    (Input|SetInputModeGameOnly self false)
    (Variables|/Script/Engine.PlayerController|SetbShowMouseCursor self false)
    (else
      (UserInterface|Viewport|AddtoViewport (Variables|Default|GetInventoryWidget) 0)
      (Input|SetInputModeGameandUI self (Variables|Default|GetInventoryWidget) "DoNotLock" false false)
      (Variables|/Script/Engine.PlayerController|SetbShowMouseCursor (Game|GetPlayerController 0) true))))

(event EventBeginPlay
  (if (Pawn|IsLocalController)
    (if (Class|GameplayStatics|ObjectIsA (.AsGS%20Main%20Menu (Utilities|Casting|CastToGS_MainMenu (Game|GetGameState))) "/Script/Engine.GameStateBase")
      ;[0.15 0.15 0.15 0.5] Spawn Main Menu HUD
      (bind _returnvalue (UserInterface|CreateWidget "/Game/UI/Widgets/WBP_MainMenu.WBP_MainMenu_C" self))
      (UserInterface|Viewport|AddtoViewport _returnvalue 0)
      (Variables|Default|SetbShowMouseCursor true)
      (Input|SetInputModeUIOnly self _returnvalue "DoNotLock" false)
      (elif (Class|GameplayStatics|ObjectIsA (.AsGS%20Level (Utilities|Casting|CastToGS_Level (Game|GetGameState))) "/Game/GameStates/GS_Level.GS_Level_C")
        ;[0.15 0.15 0.15 0.5] Spawn InGame HUD
        (bind _returnvalue_2 (UserInterface|CreateWidget "/Game/UI/Widgets/WBP_RoomHUD.WBP_RoomHUD_C" self))
        (bind _output_get (Variables|Default|SetRoomHUDRef _returnvalue_2))
        (UserInterface|Viewport|AddtoViewport _output_get 0)
        (bind _returnvalue_3 (UserInterface|CreateWidget "/Game/UI/Widgets/Inventory/Inventory_Widget.Inventory_Widget_C" self (Variables|Default|GetInventoryComponent) 1e+02))
        (Variables|Default|SetInventoryWidget _returnvalue_3)
        ;[0.15 0.15 0.15 0.5] Spawn + Init Inventory
        (bind _loadout (Default|FetchLoadout (.AsBP%20Room%20Zero%20Game%20Instance (Utilities|Casting|CastToBP_RoomZeroGameInstance (Game|GetGameInstance)))))
        (bind _valuepin (Utilities|Map|ForEachLoop(Map) _loadout)
          (:then
            (switch Utilities|FlowControl|Switch|SwitchonEItemType (.ItemType (Utilities|Struct|BreakFInventoryEntry _valuepin))
              (:NewEnumerator0
                (bind _output_get_2 (Variables|Default|SetItem%20Class "/Game/Blueprints/Items/Items/CanBePickedUp/BP_Key.BP_Key_C"))
                (Default|TryCreateandAddItemfromLoadout (Variables|Default|GetInventoryComponent) _valuepin _output_get_2)))))
        (elif (Class|GameplayStatics|ObjectIsA (.AsGS%20Lobby (Utilities|Casting|CastToGS_Lobby (Game|GetGameState))) "/Game/GameStates/GS_Lobby.GS_Lobby_C")
          ;[0.15 0.15 0.15 0.5] Spawn Lobby HUD
          (bind _returnvalue_4 (UserInterface|CreateWidget "/Game/UI/Widgets/WBP_Lobby.WBP_Lobby_C" self))
          (UserInterface|Viewport|AddtoViewport _returnvalue_4 0)
          (Input|SetInputModeUIOnly self _returnvalue_4 "DoNotLock" false))))))

(event EventOnItemPickedUp
  (params (ItemName :type Name :default "None"))
  (bind _roomhudref (Variables|Default|GetRoomHUDRef))
  (if (Utilities|IsValid _roomhudref)
    (Default|ShowKeyPickupMessage _roomhudref (Utilities|Text|ToText(Name) ItemName))))

(fn ConstructionScript)