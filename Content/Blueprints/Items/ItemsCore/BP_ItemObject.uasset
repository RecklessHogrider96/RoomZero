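; BP_ItemObject is an item data object for a grid inventory, holding an inventory entry struct (ItemData) and an item class.
; Getters expose the item ID, quantity, icon with rotation state, grid dimensions, class and full entry.
; UpdateQuantity adds the passed amount to the current quantity without clamping, rebuilds the struct with other fields copied, and returns the object itself.
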(fn GetName
  (return (.ItemID (Utilities|Struct|BreakFInventoryEntry (Variables|Default|GetItemData)))))

(fn GetQuantity
  (return (.Quantity (Utilities|Struct|BreakFInventoryEntry (Variables|Default|GetItemData)))))

(fn GetIcon
  (bind _itemdata (Variables|Default|GetItemData))
  (bind (_itemid _itemtype _quantity _weight _gridwidth _gridheight _rotated _icon) (Utilities|Struct|BreakFInventoryEntry _itemdata))
  (return _rotated _icon))

(fn GetItem
  (return (Variables|Default|GetItemData)))

(fn GetDimensions
  (bind _itemdata (Variables|Default|GetItemData))
  (return (Utilities|Struct|MakeIntPoint (.gridwidth _itemdata) (.gridheight _itemdata))))

(fn GetItemClass
  (return (Variables|Default|GetItemClass)))

(fn UpdateQuantity
  (params (Quantity :type Integer))
  (Variables|Default|SetItemData (Utilities|Struct|MakeFInventoryEntry (.itemid (Variables|Default|GetItemData)) (.itemtype (Variables|Default|GetItemData)) (+ Quantity (.quantity (Variables|Default|GetItemData))) (.weight (Variables|Default|GetItemData)) (.gridwidth (Variables|Default|GetItemData)) (.gridheight (Variables|Default|GetItemData)) (.rotated (Variables|Default|GetItemData)) (.icon (Variables|Default|GetItemData)) (.gridposition (Variables|Default|GetItemData))))
  (return self))