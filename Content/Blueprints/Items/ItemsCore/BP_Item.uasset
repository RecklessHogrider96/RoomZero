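; BP_Item is a world pickup actor that holds an ItemObject for the inventory, filled on BeginPlay from GetDefaultItemObject (empty here) when unset.
; Its Sphere overlap sets or clears itself as the player character's CurrentInteractable.
; PickupItem passes the ItemObject to the InventoryComponent reached through the character's LevelRef, and destroys the actor only if TryAddItem succeeds.
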(event OnComponentBeginOverlap(Sphere)
  (params (OverlappedComponent :type Primitive%20Component%20Object%20Reference) (OtherActor :type Actor%20Object%20Reference) (OtherComp :type Primitive%20Component%20Object%20Reference) (OtherBodyIndex :type Integer) (bFromSweep :type Boolean) (SweepResult :type Hit%20Result%20Structure%20%28by%20ref%29))
  (if (Actor|ActorHasTag OtherActor "Player")
    (bind _asbp_third_person_character (Utilities|Casting|CastToBP_ThirdPersonCharacter OtherActor))
    (Development|PrintString "This is an item!")
    (Variables|/Game/Blueprints/BP_ThirdPersonCharacter.BP_ThirdPersonCharacter_C|SetCurrentInteractable _asbp_third_person_character self)))

(event OnComponentEndOverlap(Sphere)
  (params (OverlappedComponent :type Primitive%20Component%20Object%20Reference) (OtherActor :type Actor%20Object%20Reference) (OtherComp :type Primitive%20Component%20Object%20Reference) (OtherBodyIndex :type Integer))
  (if (Actor|ActorHasTag OtherActor "Player")
    (bind _asbp_third_person_character (Utilities|Casting|CastToBP_ThirdPersonCharacter OtherActor))
    (Variables|/Game/Blueprints/BP_ThirdPersonCharacter.BP_ThirdPersonCharacter_C|SetCurrentInteractable _asbp_third_person_character 0)))

(event Custom|PickupItem
  (params (Character :type BP%20Third%20Person%20Character%20Object%20Reference))
  (bind _added (Default|TryAddItem (Variables|/Game/Blueprints/BP_LevelRoom.BP_LevelRoom_C|GetInventoryComponent (Variables|/Game/Blueprints/BP_ThirdPersonCharacter.BP_ThirdPersonCharacter_C|GetLevelRef Character)) (Variables|Private|GetItemObject)))
  (if _added
    (Actor|DestroyActor)))

(event EventBeginPlay
  (if (not (Utilities|IsValid (Variables|Private|GetItemObject)))
    (bind _itemobject (Private|GetDefaultItemObject))
    (Variables|Private|SetItemObject _itemobject)))

(fn ConstructionScript)

(fn GetDefaultItemObject
  (return 0))