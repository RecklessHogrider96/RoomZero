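; Interactable keypad item that collects an entered code and sends it to TargetToUnlock through TryUnlock.
; When ShowKeypadHUD is set, interacting toggles a WBP_Keypad widget with mouse input, and leaving range closes it.
; Button presses append digits, clear, or submit and reset the code, then refresh the keypad's display widget.
; IdentifyButton also selects the matching button mesh, which a timeline moves along Y as click feedback.
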(event Custom|ToggleKeypadWidget
  (if (and (Variables|Default|GetShowKeypadHUD) (UserInterface|Viewport|IsinViewport (Variables|Default|GetKeypadWidget)))
    ;[0.15 0.15 0.15 0.5] Remove the Keypad HUD to the Viewport
    (Widget|RemovefromParent (Variables|Default|GetKeypadWidget))
    (Input|SetInputModeGameOnly (Game|GetPlayerController 0) false)
    (Variables|/Script/Engine.PlayerController|SetbShowMouseCursor (Game|GetPlayerController 0) false)
    (else
      ;[0.15 0.15 0.15 0.5] Add the Keypad HUD to the Viewport
      (UserInterface|Viewport|AddtoViewport (Variables|Default|GetKeypadWidget) 0)
      (Input|SetInputModeGameandUI (Game|GetPlayerController 0) (Variables|Default|GetKeypadWidget) "DoNotLock" false false)
      (Variables|/Script/Engine.PlayerController|SetbShowMouseCursor (Game|GetPlayerController 0) true))))

(event Custom|OnButtonPress
  (params (ButtonPressed :type Name))
  (bind _buttonclickmesh (Variables|Default|GetButtonClickMesh))
  (bind _relativelocation (Variables|/Script/Engine.SceneComponent|GetRelativeLocation _buttonclickmesh))
  (Utilities|IdentifyButton ButtonPressed
    (:0
      (CallFunction|UpdateCode (Utilities|String|ToString(Name) ButtonPressed) :!label _label))
    (:1
      (goto _label))
    (:2
      (goto _label))
    (:3
      (goto _label))
    (:4
      (goto _label))
    (:5
      (goto _label))
    (:6
      (goto _label))
    (:7
      (goto _label))
    (:8
      (goto _label))
    (:9
      (goto _label))
    (:CLR
      (CallFunction|ClearCode :!label _label_2))
    (:OK
      (CallFunction|OnSubmitCode (Variables|Default|GetCurrentCode))
      (goto _label_2)))
  ;[0.15 0.15 0.15 0.5] Visually update the code on the Keypad's display
  (Default|UpdateCode (.AsWBP%20Keypad%20Display (Utilities|Casting|CastToWBP_KeypadDisplay (UserInterface|GetUserWidgetObject (Variables|Default|GetWBP_KeypadDisplay)))) (Utilities|Text|ToText(String) (Variables|Default|GetCurrentCode)))
  ;[0.15 0.15 0.15 0.5] Play Button Click Animation
  (bind _buttonclick (Timeline|PlayButtonClick PlayFromStart)
    (:Update
      (Transformation|SetRelativeLocation _buttonclickmesh (Math|Vector|MakeVector (.x _relativelocation) (.y _buttonclick) (.z _relativelocation)) false false))))

(event Custom|OnSubmitCode
  (params (CurrentCode :type String))
  (Class|BPIHasLockableComponent|TryUnlock(Message) (Variables|Default|GetTargetToUnlock) CurrentCode)
  (if (Variables|Default|GetShowKeypadHUD)
    (CallFunction|ToggleKeypadWidget)))

(event EventBeginPlay
  (if (Variables|Default|GetShowKeypadHUD)
    (bind _returnvalue (UserInterface|CreateWidget "/Game/UI/Widgets/Keypad/WBP_Keypad.WBP_Keypad_C"))
    (bind _output_get (Variables|Default|SetKeypadWidget _returnvalue))
    (EventDispatchers|BindEventtoOnSubmitCode _output_get (EventDispatchers|CreateEvent :!event Custom|OnSubmitCode))
    (EventDispatchers|BindEventtoOnButtonPress _output_get (EventDispatchers|CreateEvent :!event Custom|OnButtonPress))))

(event EventInteractwithItem
  (if (Variables|Default|GetShowKeypadHUD)
    (CallFunction|ToggleKeypadWidget)))

(event EventOnExitInteractableRange
  (if (Variables|Default|GetShowKeypadHUD)
    ;[0.15 0.15 0.15 0.5] Remove the Keypad HUD to the Viewport
    (Widget|RemovefromParent (Variables|Default|GetKeypadWidget))
    (Input|SetInputModeGameOnly (Game|GetPlayerController 0) false)
    (Variables|/Script/Engine.PlayerController|SetbShowMouseCursor (Game|GetPlayerController 0) false)))

(fn ConstructionScript
  (|CallParentFunction))

(fn UpdateCode
  (params (Input :type String))
  (Variables|Default|SetCurrentCode (Utilities|String|Append (Variables|Default|GetCurrentCode) Input)))

(fn ClearCode
  (Variables|Default|SetCurrentCode ""))