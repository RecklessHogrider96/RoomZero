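; BP_Door is a lockable exit door that sends the player to the main menu level once unlocked.
; When an actor tagged Player overlaps the door mesh, it calls TryUnlock with an empty code and prints whether the door opened or keys are missing.
; TryUnlock is a thin wrapper that forwards the code to BPLockableComponent, which decides the result.
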(event OnComponentBeginOverlap(DoorMesh)
  (params (OverlappedComponent :type Primitive%20Component%20Object%20Reference) (OtherActor :type Actor%20Object%20Reference) (OtherComp :type Primitive%20Component%20Object%20Reference) (OtherBodyIndex :type Integer) (bFromSweep :type Boolean) (SweepResult :type Hit%20Result%20Structure%20%28by%20ref%29))
  (if (Actor|ActorHasTag OtherActor "Player")
    (bind _isunlocked (CallFunction|TryUnlock))
    (if _isunlocked
      (Development|PrintString "Door is unlocked!")
      (Game|OpenLevel(byObjectReference) "/Game/Rooms/Level_MainMenu.Level_MainMenu")
      (else
        (Development|PrintString "You do not have all the keys!")))))

(fn ConstructionScript)

(fn TryUnlock
  (params (InputCode :type String))
  (bind _isunlocked (Default|TryUnlock (Variables|Default|GetBP_Lockable_Component) InputCode))
  (return _isunlocked))